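; Player controller for a 3D Tetris game that turns input into moves and rotations of the TetrisGameMode's current piece.
; Each input shifts the piece one Step horizontally or rotates it in roll or pitch, undoing the change if the piece overlaps.
; MoveDown stops auto-move and drops one step, repeating through a gated, delayed axis event while held.
; A blocked drop steps back and calls SetTagForCurrentPuzzle; otherwise StartMoveAgain runs.
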(event EventBeginPlay
  (bind _astetris_game_mode (Utilities|Casting|CastToTetrisGameMode (Game|GetGameMode)))
  (Variables|Default|SetAs%20Tetris%20Game%20Mode _astetris_game_mode))

(event Input|ActionEvents|InputActionMoveBack
  (params (Key :type Key%20Structure :default "None"))
  (bind _as_tetris_game_mode (Variables|Default|GetAs%20Tetris%20Game%20Mode))
  (bind _as_tetris_game_mode_2 (Variables|Default|GetAs%20Tetris%20Game%20Mode))
  (bind _currentpuzzle (Variables|/Game/Blueprints/TetrisGameMode.TetrisGameMode_C|GetCurrentPuzzle _as_tetris_game_mode))
  (bind _currentpuzzle_2 (Variables|/Game/Blueprints/TetrisGameMode.TetrisGameMode_C|GetCurrentPuzzle _as_tetris_game_mode_2))
  (bind _rootcomponent (Variables|/Script/Engine.Actor|GetRootComponent _currentpuzzle))
  (bind _relativelocation (Variables|/Script/Engine.SceneComponent|GetRelativeLocation _rootcomponent))
  (:Pressed
    (Transformation|SetRelativeLocation _rootcomponent (Math|Vector|MakeVector (.x _relativelocation) (+ (.y _relativelocation) (* (Variables|/Game/Blueprints/TetrisGameMode.TetrisGameMode_C|GetStep _as_tetris_game_mode) -1.0)) (.z _relativelocation)) false false)
    (if (Variables|/Game/Blueprints/puzzle/BP_Parent.BP_Parent_C|GetIsOverlaping _currentpuzzle_2)
      (Transformation|SetRelativeLocation _rootcomponent (Math|Vector|MakeVector (.x _relativelocation) (+ (.y _relativelocation) (Variables|/Game/Blueprints/TetrisGameMode.TetrisGameMode_C|GetStep _as_tetris_game_mode_2)) (.z _relativelocation)) false false)
      (Variables|/Game/Blueprints/puzzle/BP_Parent.BP_Parent_C|SetIsOverlaping _currentpuzzle_2 false))))

(event Input|ActionEvents|InputActionMoveForward
  (params (Key :type Key%20Structure :default "None"))
  (bind _as_tetris_game_mode (Variables|Default|GetAs%20Tetris%20Game%20Mode))
  (bind _as_tetris_game_mode_2 (Variables|Default|GetAs%20Tetris%20Game%20Mode))
  (bind _currentpuzzle (Variables|/Game/Blueprints/TetrisGameMode.TetrisGameMode_C|GetCurrentPuzzle _as_tetris_game_mode))
  (bind _currentpuzzle_2 (Variables|/Game/Blueprints/TetrisGameMode.TetrisGameMode_C|GetCurrentPuzzle _as_tetris_game_mode_2))
  (bind _rootcomponent (Variables|/Script/Engine.Actor|GetRootComponent _currentpuzzle))
  (bind _relativelocation (Variables|/Script/Engine.SceneComponent|GetRelativeLocation _rootcomponent))
  (:Pressed
    (Transformation|SetRelativeLocation _rootcomponent (Math|Vector|MakeVector (.x _relativelocation) (+ (.y _relativelocation) (Variables|/Game/Blueprints/TetrisGameMode.TetrisGameMode_C|GetStep _as_tetris_game_mode)) (.z _relativelocation)) false false)
    (if (Variables|/Game/Blueprints/puzzle/BP_Parent.BP_Parent_C|GetIsOverlaping _currentpuzzle_2)
      (Transformation|SetRelativeLocation _rootcomponent (Math|Vector|MakeVector (.x _relativelocation) (- (.y _relativelocation) (Variables|/Game/Blueprints/TetrisGameMode.TetrisGameMode_C|GetStep _as_tetris_game_mode_2)) (.z _relativelocation)) false false)
      (Variables|/Game/Blueprints/puzzle/BP_Parent.BP_Parent_C|SetIsOverlaping _currentpuzzle_2 false))))

(event Input|ActionEvents|InputActionRotateYawLeft
  (params (Key :type Key%20Structure :default "None")))

(event Input|ActionEvents|InputActionMoveRight
  (params (Key :type Key%20Structure :default "None"))
  (bind _as_tetris_game_mode (Variables|Default|GetAs%20Tetris%20Game%20Mode))
  (bind _as_tetris_game_mode_2 (Variables|Default|GetAs%20Tetris%20Game%20Mode))
  (bind _currentpuzzle (Variables|/Game/Blueprints/TetrisGameMode.TetrisGameMode_C|GetCurrentPuzzle _as_tetris_game_mode))
  (bind _currentpuzzle_2 (Variables|/Game/Blueprints/TetrisGameMode.TetrisGameMode_C|GetCurrentPuzzle _as_tetris_game_mode_2))
  (bind _rootcomponent (Variables|/Script/Engine.Actor|GetRootComponent _currentpuzzle))
  (bind _relativelocation (Variables|/Script/Engine.SceneComponent|GetRelativeLocation _rootcomponent))
  (:Pressed
    (Transformation|SetRelativeLocation _rootcomponent (Math|Vector|MakeVector (+ (.x _relativelocation) (* (Variables|/Game/Blueprints/TetrisGameMode.TetrisGameMode_C|GetStep _as_tetris_game_mode) -1.0)) (.y _relativelocation) (.z _relativelocation)) false false)
    (if (Variables|/Game/Blueprints/puzzle/BP_Parent.BP_Parent_C|GetIsOverlaping _currentpuzzle_2)
      (Transformation|SetRelativeLocation _rootcomponent (Math|Vector|MakeVector (+ (.x _relativelocation) (Variables|/Game/Blueprints/TetrisGameMode.TetrisGameMode_C|GetStep _as_tetris_game_mode_2)) (.y _relativelocation) (.z _relativelocation)) false false)
      (Variables|/Game/Blueprints/puzzle/BP_Parent.BP_Parent_C|SetIsOverlaping _currentpuzzle_2 false))))

(event Input|ActionEvents|InputActionMoveLeft
  (params (Key :type Key%20Structure :default "None"))
  (bind _as_tetris_game_mode (Variables|Default|GetAs%20Tetris%20Game%20Mode))
  (bind _as_tetris_game_mode_2 (Variables|Default|GetAs%20Tetris%20Game%20Mode))
  (bind _currentpuzzle (Variables|/Game/Blueprints/TetrisGameMode.TetrisGameMode_C|GetCurrentPuzzle _as_tetris_game_mode))
  (bind _currentpuzzle_2 (Variables|/Game/Blueprints/TetrisGameMode.TetrisGameMode_C|GetCurrentPuzzle _as_tetris_game_mode_2))
  (bind _rootcomponent (Variables|/Script/Engine.Actor|GetRootComponent _currentpuzzle))
  (bind _relativelocation (Variables|/Script/Engine.SceneComponent|GetRelativeLocation _rootcomponent))
  (:Pressed
    (Transformation|SetRelativeLocation _rootcomponent (Math|Vector|MakeVector (+ (.x _relativelocation) (Variables|/Game/Blueprints/TetrisGameMode.TetrisGameMode_C|GetStep _as_tetris_game_mode)) (.y _relativelocation) (.z _relativelocation)) false false)
    (if (Variables|/Game/Blueprints/puzzle/BP_Parent.BP_Parent_C|GetIsOverlaping _currentpuzzle_2)
      (Transformation|SetRelativeLocation _rootcomponent (Math|Vector|MakeVector (- (.x _relativelocation) (Variables|/Game/Blueprints/TetrisGameMode.TetrisGameMode_C|GetStep _as_tetris_game_mode_2)) (.y _relativelocation) (.z _relativelocation)) false false)
      (Variables|/Game/Blueprints/puzzle/BP_Parent.BP_Parent_C|SetIsOverlaping _currentpuzzle_2 false))))

(event Input|ActionEvents|InputActionRotateForward
  (params (Key :type Key%20Structure :default "None"))
  (bind _as_tetris_game_mode (Variables|Default|GetAs%20Tetris%20Game%20Mode))
  (bind _positiverotatedegree (Variables|/Game/Blueprints/TetrisGameMode.TetrisGameMode_C|GetPositiveRotateDegree _as_tetris_game_mode))
  (bind _currentpuzzle (Variables|/Game/Blueprints/TetrisGameMode.TetrisGameMode_C|GetCurrentPuzzle _as_tetris_game_mode))
  (:Pressed
    (Transformation|AddLocalRotation (Variables|/Game/Blueprints/puzzle/BP_Parent.BP_Parent_C|GetScene (Variables|/Game/Blueprints/TetrisGameMode.TetrisGameMode_C|GetCurrentPuzzle _as_tetris_game_mode)) (Math|Rotator|MakeRotator _positiverotatedegree 0.0 0.0) false false)
    (if (Variables|/Game/Blueprints/puzzle/BP_Parent.BP_Parent_C|GetIsOverlaping _currentpuzzle)
      (Transformation|AddLocalRotation (Variables|/Game/Blueprints/puzzle/BP_Parent.BP_Parent_C|GetScene _currentpuzzle) (Math|Rotator|MakeRotator (* _positiverotatedegree -1.0) 0.0 0.0) false false)
      (Variables|/Game/Blueprints/puzzle/BP_Parent.BP_Parent_C|SetIsOverlaping (Variables|/Game/Blueprints/TetrisGameMode.TetrisGameMode_C|GetCurrentPuzzle _as_tetris_game_mode) false))))

(event Input|ActionEvents|InputActionMoveDown
  (params (Key :type Key%20Structure :default "None"))
  (bind _as_tetris_game_mode (Variables|Default|GetAs%20Tetris%20Game%20Mode))
  (bind _currentpuzzle (Variables|/Game/Blueprints/TetrisGameMode.TetrisGameMode_C|GetCurrentPuzzle _as_tetris_game_mode))
  (bind _currentpuzzle_2 (Variables|/Game/Blueprints/TetrisGameMode.TetrisGameMode_C|GetCurrentPuzzle _as_tetris_game_mode))
  (bind _rootcomponent (Variables|/Script/Engine.Actor|GetRootComponent _currentpuzzle))
  (bind _relativelocation (Variables|/Script/Engine.SceneComponent|GetRelativeLocation _rootcomponent))
  (:Pressed
    (Utilities|FlowControl|Sequence
      (:then_0
        (Utilities|FlowControl|Gate true) ; enters at Open
      )
      (:then_1
        (Default|StopAutoMove _as_tetris_game_mode)
        (Transformation|SetRelativeLocation _rootcomponent (Math|Vector|MakeVector (.x _relativelocation) (.y _relativelocation) (+ (.z _relativelocation) (* (Variables|/Game/Blueprints/TetrisGameMode.TetrisGameMode_C|GetStep _as_tetris_game_mode) -1.0))) false false)
        (if (Variables|/Game/Blueprints/puzzle/BP_Parent.BP_Parent_C|GetIsOverlaping _currentpuzzle_2)
          (Transformation|SetRelativeLocation (Variables|/Script/Engine.Actor|GetRootComponent _currentpuzzle_2) (Math|Vector|MakeVector (.x _relativelocation) (.y _relativelocation) (+ (.z _relativelocation) (Variables|/Game/Blueprints/TetrisGameMode.TetrisGameMode_C|GetStep (Variables|Default|GetAs%20Tetris%20Game%20Mode)))) false false)
          (Variables|/Game/Blueprints/puzzle/BP_Parent.BP_Parent_C|SetIsOverlaping _currentpuzzle_2 false)
          (Default|SetTagforCurrentPuzzle (Variables|Default|GetAs%20Tetris%20Game%20Mode))
          (else
            (Default|StartMoveAgain _as_tetris_game_mode))))))
  (:Released
    (Utilities|FlowControl|Gate true) ; enters at Close
  ))

(event Input|ActionEvents|InputActionRotateBack
  (params (Key :type Key%20Structure :default "None"))
  (bind _as_tetris_game_mode (Variables|Default|GetAs%20Tetris%20Game%20Mode))
  (bind _negativerotatedegree (Variables|/Game/Blueprints/TetrisGameMode.TetrisGameMode_C|GetNegativeRotateDegree _as_tetris_game_mode))
  (bind _currentpuzzle (Variables|/Game/Blueprints/TetrisGameMode.TetrisGameMode_C|GetCurrentPuzzle _as_tetris_game_mode))
  (:Pressed
    (Transformation|AddLocalRotation (Variables|/Game/Blueprints/puzzle/BP_Parent.BP_Parent_C|GetScene (Variables|/Game/Blueprints/TetrisGameMode.TetrisGameMode_C|GetCurrentPuzzle _as_tetris_game_mode)) (Math|Rotator|MakeRotator _negativerotatedegree 0.0 0.0) false false)
    (if (Variables|/Game/Blueprints/puzzle/BP_Parent.BP_Parent_C|GetIsOverlaping _currentpuzzle)
      (Transformation|AddLocalRotation (Variables|/Game/Blueprints/puzzle/BP_Parent.BP_Parent_C|GetScene _currentpuzzle) (Math|Rotator|MakeRotator (* _negativerotatedegree -1.0) 0.0 0.0) false false)
      (Variables|/Game/Blueprints/puzzle/BP_Parent.BP_Parent_C|SetIsOverlaping (Variables|/Game/Blueprints/TetrisGameMode.TetrisGameMode_C|GetCurrentPuzzle _as_tetris_game_mode) false))))

(event Input|ActionEvents|InputActionRotateRight
  (params (Key :type Key%20Structure :default "None"))
  (bind _as_tetris_game_mode (Variables|Default|GetAs%20Tetris%20Game%20Mode))
  (bind _positiverotatedegree (Variables|/Game/Blueprints/TetrisGameMode.TetrisGameMode_C|GetPositiveRotateDegree _as_tetris_game_mode))
  (bind _currentpuzzle (Variables|/Game/Blueprints/TetrisGameMode.TetrisGameMode_C|GetCurrentPuzzle _as_tetris_game_mode))
  (:Pressed
    (Transformation|AddLocalRotation (Variables|/Game/Blueprints/puzzle/BP_Parent.BP_Parent_C|GetScene (Variables|/Game/Blueprints/TetrisGameMode.TetrisGameMode_C|GetCurrentPuzzle _as_tetris_game_mode)) (Math|Rotator|MakeRotator 0.0 _positiverotatedegree 0.0) false false)
    (if (Variables|/Game/Blueprints/puzzle/BP_Parent.BP_Parent_C|GetIsOverlaping _currentpuzzle)
      (Transformation|AddLocalRotation (Variables|/Game/Blueprints/puzzle/BP_Parent.BP_Parent_C|GetScene _currentpuzzle) (Math|Rotator|MakeRotator 0.0 (* _positiverotatedegree -1.0) 0.0) false false)
      (Variables|/Game/Blueprints/puzzle/BP_Parent.BP_Parent_C|SetIsOverlaping (Variables|/Game/Blueprints/TetrisGameMode.TetrisGameMode_C|GetCurrentPuzzle _as_tetris_game_mode) false))))

(event Input|ActionEvents|InputActionRotateLeft
  (params (Key :type Key%20Structure :default "None"))
  (bind _as_tetris_game_mode (Variables|Default|GetAs%20Tetris%20Game%20Mode))
  (bind _negativerotatedegree (Variables|/Game/Blueprints/TetrisGameMode.TetrisGameMode_C|GetNegativeRotateDegree _as_tetris_game_mode))
  (bind _currentpuzzle (Variables|/Game/Blueprints/TetrisGameMode.TetrisGameMode_C|GetCurrentPuzzle _as_tetris_game_mode))
  (:Pressed
    (Transformation|AddLocalRotation (Variables|/Game/Blueprints/puzzle/BP_Parent.BP_Parent_C|GetScene (Variables|/Game/Blueprints/TetrisGameMode.TetrisGameMode_C|GetCurrentPuzzle _as_tetris_game_mode)) (Math|Rotator|MakeRotator 0.0 _negativerotatedegree 0.0) false false)
    (if (Variables|/Game/Blueprints/puzzle/BP_Parent.BP_Parent_C|GetIsOverlaping _currentpuzzle)
      (Transformation|AddLocalRotation (Variables|/Game/Blueprints/puzzle/BP_Parent.BP_Parent_C|GetScene _currentpuzzle) (Math|Rotator|MakeRotator 0.0 (* _negativerotatedegree -1.0) 0.0) false false)
      (Variables|/Game/Blueprints/puzzle/BP_Parent.BP_Parent_C|SetIsOverlaping (Variables|/Game/Blueprints/TetrisGameMode.TetrisGameMode_C|GetCurrentPuzzle _as_tetris_game_mode) false))))

(event Input|ActionEvents|InputActionRotateYawRight
  (params (Key :type Key%20Structure :default "None")))

(event Input|AxisEvents|InputAxisMoveDown
  (params (AxisValue :type Float%20%28single-precision%29))
  (bind _as_tetris_game_mode (Variables|Default|GetAs%20Tetris%20Game%20Mode))
  (bind _currentpuzzle (Variables|/Game/Blueprints/TetrisGameMode.TetrisGameMode_C|GetCurrentPuzzle _as_tetris_game_mode))
  (bind _currentpuzzle_2 (Variables|/Game/Blueprints/TetrisGameMode.TetrisGameMode_C|GetCurrentPuzzle _as_tetris_game_mode))
  (bind _rootcomponent (Variables|/Script/Engine.Actor|GetRootComponent _currentpuzzle))
  (bind _relativelocation (Variables|/Script/Engine.SceneComponent|GetRelativeLocation _rootcomponent))
  (Utilities|FlowControl|Delay 0.1)
  (Utilities|FlowControl|Gate true
    (:Exit
      (if (> (Class|PlayerController|GetInputKeyTimeDown (Game|GetPlayerController 0) (stale Input|ActionEvents|InputActionMoveDown Key)) 0.3)
        (Default|StopAutoMove _as_tetris_game_mode)
        (Transformation|SetRelativeLocation _rootcomponent (Math|Vector|MakeVector (.x _relativelocation) (.y _relativelocation) (+ (.z _relativelocation) (* (Variables|/Game/Blueprints/TetrisGameMode.TetrisGameMode_C|GetStep _as_tetris_game_mode) -1.0))) false false)
        (if (Variables|/Game/Blueprints/puzzle/BP_Parent.BP_Parent_C|GetIsOverlaping _currentpuzzle_2)
          (Transformation|SetRelativeLocation (Variables|/Script/Engine.Actor|GetRootComponent _currentpuzzle_2) (Math|Vector|MakeVector (.x _relativelocation) (.y _relativelocation) (+ (.z _relativelocation) (Variables|/Game/Blueprints/TetrisGameMode.TetrisGameMode_C|GetStep (Variables|Default|GetAs%20Tetris%20Game%20Mode)))) false false)
          (Variables|/Game/Blueprints/puzzle/BP_Parent.BP_Parent_C|SetIsOverlaping _currentpuzzle_2 false)
          (Default|SetTagforCurrentPuzzle (Variables|Default|GetAs%20Tetris%20Game%20Mode))
          (else
            (Default|StartMoveAgain _as_tetris_game_mode)))))))

(fn ConstructionScript)