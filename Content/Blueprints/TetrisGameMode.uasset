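; Tetris game mode that spawns random pieces at StartLine, drives their automatic fall and handles block removal.
; The TimeDown timeline's Finished event lowers the current piece by Step, backing up on overlap to tag it PuzzleGround and spawn the next.
; DestroyComponent removes given blocks and emptied actors through cast chains over seven piece classes, lowers every PuzzleGround piece one Step, then resumes the fall.
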(event Custom|StopAutoMove
  (bind _currentpuzzle (Variables|Default|GetCurrentPuzzle))
  (bind _currentpuzzle_2 (Variables|Default|GetCurrentPuzzle))
  (bind _rootcomponent (Variables|/Script/Engine.Actor|GetRootComponent _currentpuzzle_2))
  (bind _relativelocation (Variables|/Script/Engine.SceneComponent|GetRelativeLocation _rootcomponent))
  (Timeline|TimeDown Stop
    (:Finished
      (Transformation|SetRelativeLocation _rootcomponent (Math|Vector|MakeVector (.x _relativelocation) (.y _relativelocation) (+ (.z _relativelocation) (* (Variables|Default|GetStep) -1.0))) false false)
      (if (Variables|/Game/Blueprints/puzzle/BP_Parent.BP_Parent_C|GetIsOverlaping _currentpuzzle)
        (Transformation|SetRelativeLocation (Variables|/Script/Engine.Actor|GetRootComponent _currentpuzzle) (Math|Vector|MakeVector (.x _relativelocation) (.y _relativelocation) (+ (.z _relativelocation) (Variables|Default|GetStep))) false false)
        (Variables|/Game/Blueprints/puzzle/BP_Parent.BP_Parent_C|SetIsOverlaping _currentpuzzle false)
        (CallFunction|SetTagandSpawnforCurrentPuzzle)
        (else
          (Timeline|TimeDown ReverseFromEnd))))))

(event Custom|Set%20Tags%20For%20Current%20Puzzle
  (Variables|/Script/Engine.Actor|SetTags (Variables|Default|GetCurrentPuzzle) (Utilities|Array|MakeArray "PuzzleGround")))

(event Custom|StartMoveAgain
  (bind _currentpuzzle (Variables|Default|GetCurrentPuzzle))
  (bind _currentpuzzle_2 (Variables|Default|GetCurrentPuzzle))
  (bind _rootcomponent (Variables|/Script/Engine.Actor|GetRootComponent _currentpuzzle_2))
  (bind _relativelocation (Variables|/Script/Engine.SceneComponent|GetRelativeLocation _rootcomponent))
  (Timeline|TimeDown PlayFromStart
    (:Finished
      (Transformation|SetRelativeLocation _rootcomponent (Math|Vector|MakeVector (.x _relativelocation) (.y _relativelocation) (+ (.z _relativelocation) (* (Variables|Default|GetStep) -1.0))) false false)
      (if (Variables|/Game/Blueprints/puzzle/BP_Parent.BP_Parent_C|GetIsOverlaping _currentpuzzle)
        (Transformation|SetRelativeLocation (Variables|/Script/Engine.Actor|GetRootComponent _currentpuzzle) (Math|Vector|MakeVector (.x _relativelocation) (.y _relativelocation) (+ (.z _relativelocation) (Variables|Default|GetStep))) false false)
        (Variables|/Game/Blueprints/puzzle/BP_Parent.BP_Parent_C|SetIsOverlaping _currentpuzzle false)
        (CallFunction|SetTagandSpawnforCurrentPuzzle)
        (else
          (Timeline|TimeDown ReverseFromEnd))))))

(event Custom|Set%20Tag%20And%20Spawn%20for%20current%20puzzle
  (bind _currentpuzzle (Variables|Default|GetCurrentPuzzle))
  (bind _currentpuzzle_2 (Variables|Default|GetCurrentPuzzle))
  (bind _rootcomponent (Variables|/Script/Engine.Actor|GetRootComponent _currentpuzzle_2))
  (bind _relativelocation (Variables|/Script/Engine.SceneComponent|GetRelativeLocation _rootcomponent))
  (Variables|/Script/Engine.Actor|SetTags (Variables|Default|GetCurrentPuzzle) (Utilities|Array|MakeArray "PuzzleGround"))
  (bind _returnvalue (Game|SpawnActorfromClass (.OutItem (Utilities|Array|Random (Variables|Default|GetActorList))) (Math|Transform|MakeTransform (.location (Variables|Default|GetStartLine)) "0, 0, 0" "1.000000,1.000000,1.000000") "AlwaysSpawn" 0 0))
  (CallFunction|DynamicCastandSetCurrentPuzzle _returnvalue)
  (Timeline|TimeDown PlayFromStart
    (:Finished
      (Transformation|SetRelativeLocation _rootcomponent (Math|Vector|MakeVector (.x _relativelocation) (.y _relativelocation) (+ (.z _relativelocation) (* (Variables|Default|GetStep) -1.0))) false false)
      (if (Variables|/Game/Blueprints/puzzle/BP_Parent.BP_Parent_C|GetIsOverlaping _currentpuzzle)
        (Transformation|SetRelativeLocation (Variables|/Script/Engine.Actor|GetRootComponent _currentpuzzle) (Math|Vector|MakeVector (.x _relativelocation) (.y _relativelocation) (+ (.z _relativelocation) (Variables|Default|GetStep))) false false)
        (Variables|/Game/Blueprints/puzzle/BP_Parent.BP_Parent_C|SetIsOverlaping _currentpuzzle false)
        (CallFunction|SetTagandSpawnforCurrentPuzzle)
        (else
          (Timeline|TimeDown ReverseFromEnd))))))

(event Custom|Event%20Destroy%20Component
  (params (OverlapedComponent :type Array%20of%20Primitive%20Component%20Object%20References))
  (for _array_element OverlapedComponent
    (CallFunction|DestroyComponentbyPuzzle (Components|GetOwner _array_element) _array_element))
  (CallFunction|EventMoveActorDown))

(event Custom|Event%20Move%20Actor%20Down
  (bind _outactors (Actor|GetAllActorsOfClasswithTag "/Game/Blueprints/puzzle/BP_Parent.BP_Parent_C" "PuzzleGround"))
  (for _array_element _outactors
    (Transformation|SetRelativeLocation (Variables|/Script/Engine.Actor|GetRootComponent _array_element) (Math|Vector|MakeVector (.x (Variables|/Script/Engine.SceneComponent|GetRelativeLocation (Variables|/Script/Engine.Actor|GetRootComponent _array_element))) (.y (Variables|/Script/Engine.SceneComponent|GetRelativeLocation (Variables|/Script/Engine.Actor|GetRootComponent _array_element))) (- (.z (Variables|/Script/Engine.SceneComponent|GetRelativeLocation (Variables|/Script/Engine.Actor|GetRootComponent _array_element))) (Variables|Default|GetStep))) false false))
  (CallFunction|StartMoveAgain))

(event EventBeginPlay
  (bind _currentpuzzle (Variables|Default|GetCurrentPuzzle))
  (bind _currentpuzzle_2 (Variables|Default|GetCurrentPuzzle))
  (bind _rootcomponent (Variables|/Script/Engine.Actor|GetRootComponent _currentpuzzle_2))
  (bind _relativelocation (Variables|/Script/Engine.SceneComponent|GetRelativeLocation _rootcomponent))
  (bind _returnvalue (Game|SpawnActorfromClass (.OutItem (Utilities|Array|Random (Variables|Default|GetActorList))) (Math|Transform|MakeTransform (.location (Variables|Default|GetStartLine)) "0, 0, 0" "1.000000,1.000000,1.000000") "AlwaysSpawn" 0 0))
  (CallFunction|DynamicCastandSetCurrentPuzzle _returnvalue)
  (Timeline|TimeDown PlayFromStart
    (:Finished
      (Transformation|SetRelativeLocation _rootcomponent (Math|Vector|MakeVector (.x _relativelocation) (.y _relativelocation) (+ (.z _relativelocation) (* (Variables|Default|GetStep) -1.0))) false false)
      (if (Variables|/Game/Blueprints/puzzle/BP_Parent.BP_Parent_C|GetIsOverlaping _currentpuzzle)
        (Transformation|SetRelativeLocation (Variables|/Script/Engine.Actor|GetRootComponent _currentpuzzle) (Math|Vector|MakeVector (.x _relativelocation) (.y _relativelocation) (+ (.z _relativelocation) (Variables|Default|GetStep))) false false)
        (Variables|/Game/Blueprints/puzzle/BP_Parent.BP_Parent_C|SetIsOverlaping _currentpuzzle false)
        (CallFunction|SetTagandSpawnforCurrentPuzzle)
        (else
          (Timeline|TimeDown ReverseFromEnd))))))

(fn ConstructionScript)

(fn DestroyComponentbyPuzzle
  (params (Actor%20Object%20 :type Actor%20Object%20Reference) (Component :type Primitive%20Component%20Object%20Reference))
  (bind _asbp_i_child (Utilities|Casting|CastToBP_I_Child Actor%20Object%20)
    (:then
      (Default|EventDestroyComponentfromActor _asbp_i_child Component)
      (if (== (Utilities|Array|Length (Components|GetChildrenComponents (Variables|/Game/Blueprints/puzzle/BP_Parent.BP_Parent_C|GetScene _asbp_i_child) true)) 0)
        (Actor|DestroyActor _asbp_i_child)))
    (:CastFailed
      (bind _asbp_j_child (Utilities|Casting|CastToBP_J_Child Actor%20Object%20)
        (:then
          (Default|EventDestroyComponentfromActor _asbp_j_child Component)
          (if (== (Utilities|Array|Length (Components|GetChildrenComponents (Variables|/Game/Blueprints/puzzle/BP_Parent.BP_Parent_C|GetScene _asbp_j_child) true)) 0)
            (Actor|DestroyActor _asbp_j_child)))
        (:CastFailed
          (bind _asbp_o_child (Utilities|Casting|CastToBP_O_Child Actor%20Object%20)
            (:then
              (Default|EventDestroyComponentfromActor _asbp_o_child Component)
              (if (== (Utilities|Array|Length (Components|GetChildrenComponents (Variables|/Game/Blueprints/puzzle/BP_Parent.BP_Parent_C|GetScene _asbp_o_child) true)) 0)
                (Actor|DestroyActor _asbp_o_child)))
            (:CastFailed
              (bind _asbp_s_child (Utilities|Casting|CastToBP_S_Child Actor%20Object%20)
                (:then
                  (Default|EventDestroyComponentfromActor _asbp_s_child Component)
                  (if (== (Utilities|Array|Length (Components|GetChildrenComponents (Variables|/Game/Blueprints/puzzle/BP_Parent.BP_Parent_C|GetScene _asbp_s_child) true)) 0)
                    (Actor|DestroyActor _asbp_s_child)))
                (:CastFailed
                  (bind _asbp_z_child (Utilities|Casting|CastToBP_Z_Child Actor%20Object%20)
                    (:then
                      (Default|EventDestroyComponentfromActor _asbp_z_child Component)
                      (if (== (Utilities|Array|Length (Components|GetChildrenComponents (Variables|/Game/Blueprints/puzzle/BP_Parent.BP_Parent_C|GetScene _asbp_z_child) true)) 0)
                        (Actor|DestroyActor _asbp_z_child)))
                    (:CastFailed
                      (bind _asbp_l_child (Utilities|Casting|CastToBP_L_Child Actor%20Object%20)
                        (:then
                          (Default|EventDestroyComponentfromActor _asbp_l_child Component)
                          (if (== (Utilities|Array|Length (Components|GetChildrenComponents (Variables|/Game/Blueprints/puzzle/BP_Parent.BP_Parent_C|GetScene _asbp_l_child) true)) 0)
                            (Actor|DestroyActor _asbp_l_child)))
                        (:CastFailed
                          (bind _asbp_t_child (Utilities|Casting|CastToBP_T_Child Actor%20Object%20))
                          (Default|EventDestroyComponentfromActor _asbp_t_child Component)
                          (if (== (Utilities|Array|Length (Components|GetChildrenComponents (Variables|/Game/Blueprints/puzzle/BP_Parent.BP_Parent_C|GetScene _asbp_t_child) true)) 0)
                            (Actor|DestroyActor _asbp_t_child)))))))))))))))

(fn DynamicCastandSetCurrentPuzzle
  (params (Actor :type Actor%20Object%20Reference))
  (bind _asbp_i_child (Utilities|Casting|CastToBP_I_Child Actor)
    (:then
      (Variables|Default|SetCurrentPuzzle _asbp_i_child))
    (:CastFailed
      (bind _asbp_j_child (Utilities|Casting|CastToBP_J_Child Actor)
        (:then
          (Variables|Default|SetCurrentPuzzle _asbp_j_child))
        (:CastFailed
          (bind _asbp_o_child (Utilities|Casting|CastToBP_O_Child Actor)
            (:then
              (Variables|Default|SetCurrentPuzzle _asbp_o_child))
            (:CastFailed
              (bind _asbp_s_child (Utilities|Casting|CastToBP_S_Child Actor)
                (:then
                  (Variables|Default|SetCurrentPuzzle _asbp_s_child))
                (:CastFailed
                  (bind _asbp_z_child (Utilities|Casting|CastToBP_Z_Child Actor)
                    (:then
                      (Variables|Default|SetCurrentPuzzle _asbp_z_child))
                    (:CastFailed
                      (bind _asbp_l_child (Utilities|Casting|CastToBP_L_Child Actor)
                        (:then
                          (Variables|Default|SetCurrentPuzzle _asbp_l_child))
                        (:CastFailed
                          (bind _asbp_t_child (Utilities|Casting|CastToBP_T_Child Actor))
                          (Variables|Default|SetCurrentPuzzle _asbp_t_child))))))))))))))