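; Base Blueprint for puzzle pieces built from four cube components, with shared helpers and overlap detection.
; Any cube's begin overlap sets IsOverlaping, and custom events switch component mobility, disable tick or destroy components.
; CalculateVectorDistance line-traces from a point down and along both horizontal axes, returning five hit distances plus the downward hit component.
; The event graph's per-cube minimum-distance logic and the debug drawing are disconnected.
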(event OnComponentBeginOverlap(Cube3)
  (params (OverlappedComponent :type Primitive%20Component%20Object%20Reference) (OtherActor :type Actor%20Object%20Reference) (OtherComp :type Primitive%20Component%20Object%20Reference) (OtherBodyIndex :type Integer) (bFromSweep :type Boolean) (SweepResult :type Hit%20Result%20Structure%20%28by%20ref%29))
  ;[1 1 1] Check When Puzzle Is Overlaping Anything
  (Variables|Default|SetIsOverlaping true))

(event OnComponentBeginOverlap(Cube)
  (params (OverlappedComponent :type Primitive%20Component%20Object%20Reference) (OtherActor :type Actor%20Object%20Reference) (OtherComp :type Primitive%20Component%20Object%20Reference) (OtherBodyIndex :type Integer) (bFromSweep :type Boolean) (SweepResult :type Hit%20Result%20Structure%20%28by%20ref%29))
  ;[1 1 1] Check When Puzzle Is Overlaping Anything
  (Variables|Default|SetIsOverlaping true))

(event OnComponentBeginOverlap(Cube2)
  (params (OverlappedComponent :type Primitive%20Component%20Object%20Reference) (OtherActor :type Actor%20Object%20Reference) (OtherComp :type Primitive%20Component%20Object%20Reference) (OtherBodyIndex :type Integer) (bFromSweep :type Boolean) (SweepResult :type Hit%20Result%20Structure%20%28by%20ref%29))
  ;[1 1 1] Check When Puzzle Is Overlaping Anything
  (Variables|Default|SetIsOverlaping true))

(event OnComponentBeginOverlap(Cube1)
  (params (OverlappedComponent :type Primitive%20Component%20Object%20Reference) (OtherActor :type Actor%20Object%20Reference) (OtherComp :type Primitive%20Component%20Object%20Reference) (OtherBodyIndex :type Integer) (bFromSweep :type Boolean) (SweepResult :type Hit%20Result%20Structure%20%28by%20ref%29))
  ;[1 1 1] Check When Puzzle Is Overlaping Anything
  (Variables|Default|SetIsOverlaping true))

(event Custom|Event%20Destroy%20Component%20from%20actor
  (params (Target :type Actor%20Component%20Object%20Reference))
  ;[1 1 1] Destroy Component By list of component
  (Components|DestroyComponent Target))

(event Custom|Set%20Movable%20for%20Puzzle
  (params (ChildrenComponent :type Array%20of%20Scene%20Component%20Object%20References))
  (Utilities|Array|SetArrayElem ChildrenComponent (+ (Utilities|Array|LastIndex ChildrenComponent) 1) (Variables|Default|GetDefaultSceneRoot) true)
  (Transformation|SetMobility ChildrenComponent "Movable"))

(event Custom|SetEventTickDisable
  (Actor|Tick|SetActorTickEnabled false))

(event Custom|set%20Static%20for%20Puzzle%20by%20component
  (params (ChildrenComponent :type Array%20of%20Scene%20Component%20Object%20References))
  (Utilities|Array|SetArrayElem ChildrenComponent (+ (Utilities|Array|LastIndex ChildrenComponent) 1) (Variables|Default|GetDefaultSceneRoot) true)
  (Transformation|SetMobility ChildrenComponent "Static"))

(event Collision|EventActorBeginOverlap
  (params (OtherActor :type Actor%20Object%20Reference)))

(event EventTick
  (params (DeltaSeconds :type Float%20%28single-precision%29))
  ;[1 1 1] Trash code
)

(fn ConstructionScript)

(fn CalculateVectorDistance
  (params (InVec :type Vector) (ObjectTypes :type Array%20of%20EObjectTypeQuery%20Enums :default "ObjectTypeQuery1") (bIgnoreSelf :type Boolean) (ActorsToIgnore :type Array%20of%20Actor%20Object%20References))
  (bind (_x _y _z) (Math|Vector|BreakVector InVec))
  (bind (_x_2 _y_2 _z_2) (Math|Vector|BreakVector InVec))
  (bind (_x_3 _y_3 _z_3) (Math|Vector|BreakVector InVec))
  (bind (_x_4 _y_4 _z_4) (Math|Vector|BreakVector InVec))
  (bind (_x_5 _y_5 _z_5) (Math|Vector|BreakVector InVec))
  (bind _outhit (Collision|LineTraceForObjects InVec (Math|Vector|MakeVector _x_3 _y_3 (* _z_3 -3e+03)) ObjectTypes false ActorsToIgnore "None" bIgnoreSelf))
  (bind _outhit_2 (Collision|LineTraceForObjects InVec (Math|Vector|MakeVector (* (Math|Float|Absolute(Float) (* (+ _x_2 1.0) -3e+03)) -1.0) _y_2 _z_2) ObjectTypes false ActorsToIgnore "None" bIgnoreSelf))
  (bind _outhit_3 (Collision|LineTraceForObjects InVec (Math|Vector|MakeVector _x_4 (* (Math|Float|Absolute(Float) (* (+ _y_4 1.0) -3e+03)) -1.0) _z_4) ObjectTypes false ActorsToIgnore "None" bIgnoreSelf))
  (bind _outhit_4 (Collision|LineTraceForObjects InVec (Math|Vector|MakeVector (Math|Float|Absolute(Float) (* (+ _x_5 1.0) 3e+03)) _y_5 _z_5) ObjectTypes false ActorsToIgnore "None" bIgnoreSelf))
  (bind _outhit_5 (Collision|LineTraceForObjects InVec (Math|Vector|MakeVector _x (Math|Float|Absolute(Float) (* (+ _y 1.0) 3e+03)) _z) ObjectTypes false ActorsToIgnore "None" bIgnoreSelf))
  (return (.Distance (Collision|BreakHitResult _outhit)) (.Distance (Collision|BreakHitResult _outhit_2)) (.Distance (Collision|BreakHitResult _outhit_3)) (.Distance (Collision|BreakHitResult _outhit_4)) (.Distance (Collision|BreakHitResult _outhit_5)) (.HitComponent (Collision|BreakHitResult _outhit))))